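; Dynamic water volume that renders waterline geometry through a scene capture snapped to the player camera.
; The capture shows only the waterline cube and top/bottom blocks, which are hidden from the owning player.
; Timelines keep feeding the second found WaterBody_BP0's height texture into the cube and top-block materials.
; Box overlaps toggle capture visibility to save FPS, while cube overlaps toggle custom depth on overlapping components.
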(event `self.ReceiveBeginPlay`
  (bind _waterlinecube (`self.WaterlineCube`))
  (bind _blocktop (`self.BlockTop`))
  (`|ExecutionSequence`
    (:`then_0`
      (for _array_element (`|MakeArray` (`self.WaterlineCube`) (`self.BlockTop`) (`self.BlockBottom`) :!type "PrimitiveComponent Object Reference")
        (`SceneCaptureComponent.ShowOnlyComponent` (`self.SceneCaptureComponent2D`) _array_element))
      (`self.SetOwner` (`GameplayStatics.GetPlayerCharacter` 0))
      (`PrimitiveComponent.SetOwnerNoSee` (`self.WaterlineCube`) true)
      (`PrimitiveComponent.SetOwnerNoSee` (`self.BlockBottom`) true)
      (`PrimitiveComponent.SetOwnerNoSee` (`self.BlockTop`) true)
      (`|ExecutionSequence`
        (:`then_0`
          (bind _returnvalue (`PrimitiveComponent.CreateDynamicMaterialInstance` _waterlinecube 0 "/Game/_Marvelmaster_Waterline_and_Volume/Materials/Y_DynamicWaterVolume/Y_ShowVolumeDynamic_mat.Y_ShowVolumeDynamic_mat" "None"))
          (bind _output_get (set `self.dynmatcube` _returnvalue))
          (`PrimitiveComponent.SetMaterial` _waterlinecube 0 _output_get)
          (bind _outactors (`GameplayStatics.GetAllActorsOfClass` "/Game/_Marvelmaster_infinite_reactive_water_/Blueprints/WaterBody_BP0.WaterBody_BP0_C"))
          ;[1 1 1] for some reason needs to update all the time in packed project
          (`Timeline|Timeline_0` :!via `PlayFromStart`
            (:`Update`
              (`MaterialInstanceDynamic.SetTextureParameterValue` (`self.dynmatcube`) "Heightfield" (`/Game/_Marvelmaster_infinite_reactive_water_/Blueprints/WaterBody_BP0.height` (`|GetArrayItem` _outactors 1))))))
        (:`then_1`
          (bind _returnvalue_2 (`PrimitiveComponent.CreateDynamicMaterialInstance` _blocktop 0 "/Game/_Marvelmaster_Waterline_and_Volume/Materials/Y_DynamicWaterVolume/Y_HideVolumeDynamic_mat.Y_HideVolumeDynamic_mat" "None"))
          (bind _output_get_2 (set `self.dynmattop` _returnvalue_2))
          (`PrimitiveComponent.SetMaterial` _blocktop 0 _output_get_2)
          (bind _outactors_2 (`GameplayStatics.GetAllActorsOfClass` "/Game/_Marvelmaster_infinite_reactive_water_/Blueprints/WaterBody_BP0.WaterBody_BP0_C"))
          (`Timeline|Timeline_1` :!via `PlayFromStart`
            (:`Update`
              (`MaterialInstanceDynamic.SetTextureParameterValue` (`self.dynmattop`) "Heightfield" (`/Game/_Marvelmaster_infinite_reactive_water_/Blueprints/WaterBody_BP0.height` (`|GetArrayItem` _outactors_2 1))))))))
    (:`then_1`
      (`SceneComponent.K2_AttachToComponent` (`self.SceneCaptureComponent2D`) (`PlayerCameraManager.TransformComponent` (`PlayerController.PlayerCameraManager` (`GameplayStatics.GetPlayerController` 0))) "None" "SnapToTarget" "SnapToTarget" "SnapToTarget" true))))

(event `self.ReceiveTick`
  (params (DeltaSeconds :type "Float (single-precision)")))

(event `self.WaterlineCube.OnComponentBeginOverlap`
  (params (OverlappedComponent :type "PrimitiveComponent Object Reference") (OtherActor :type "Actor Object Reference") (OtherComp :type "PrimitiveComponent Object Reference") (OtherBodyIndex :type Integer) (bFromSweep :type Boolean) (SweepResult :type "HitResult Structure (by ref)"))
  (`PrimitiveComponent.SetRenderCustomDepth` OtherComp false)
  (`KismetSystemLibrary.PrintString` "Custom Depth disabled"))

(event `self.WaterlineCube.OnComponentEndOverlap`
  (params (OverlappedComponent :type "PrimitiveComponent Object Reference") (OtherActor :type "Actor Object Reference") (OtherComp :type "PrimitiveComponent Object Reference") (OtherBodyIndex :type Integer))
  (`PrimitiveComponent.SetRenderCustomDepth` OtherComp true)
  (`KismetSystemLibrary.PrintString` "Custom Depth enabled"))

(event `self.Box.OnComponentBeginOverlap`
  (params (OverlappedComponent :type "PrimitiveComponent Object Reference") (OtherActor :type "Actor Object Reference") (OtherComp :type "PrimitiveComponent Object Reference") (OtherBodyIndex :type Integer) (bFromSweep :type Boolean) (SweepResult :type "HitResult Structure (by ref)"))
  ;[1 0 0.004263] deactivate capture when not in range otherwise FPS get realy low levelwide
  ; SceneCapture is initially  set to hidden in blueprint
  (`SceneComponent.SetHiddenInGame` (`self.SceneCaptureComponent2D`) false false))

(event `self.Box.OnComponentEndOverlap`
  (params (OverlappedComponent :type "PrimitiveComponent Object Reference") (OtherActor :type "Actor Object Reference") (OtherComp :type "PrimitiveComponent Object Reference") (OtherBodyIndex :type Integer))
  ;[1 0 0.004263] deactivate capture when not in range otherwise FPS get realy low levelwide
  ; SceneCapture is initially  set to hidden in blueprint
  (`SceneComponent.SetHiddenInGame` (`self.SceneCaptureComponent2D`) true false))

(fn `UserConstructionScript`
  ;[1 1 1] Flicker Debug
  (`PrimitiveComponent.SetBoundsScale` (`self.WaterlineCube`) 100.0))