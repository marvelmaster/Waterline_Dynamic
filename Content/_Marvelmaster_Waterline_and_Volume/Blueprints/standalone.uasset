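; Camera waterline actor that positions an underwater cube at the view to draw the water surface split.
; A fast timer moves the cube with a camera-attached clip-plane offsetter, switching between following camera height and water level, collapsing it high above water.
; The cube's dynamic material receives the first water body's heightfield.
; A show-only scene capture activates near the camera and clears its render target when far, allowing multiple instances.
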(event `self.ReceiveBeginPlay`
  (bind _clipplaneoffsetter (`self.ClipPlaneOffsetter`))
  (bind _underwatercube (`self.UnderWaterCube`))
  (`|ExecutionSequence`
    (:`then_0`
      (bind _aswater_tpcharacter (cast `/Game/_Marvelmaster_infinite_reactive_water_/ThirdPersonBP/Blueprints/WaterTPCharacter` (`GameplayStatics.GetPlayerCharacter` 0)))
      (set `self.Character` _aswater_tpcharacter)
      (`SceneCaptureComponent.ShowOnlyComponent` (`self.WaveCapture`) _underwatercube)
      (`self.SetOwner` (`GameplayStatics.GetPlayerCharacter` 0))
      (`PrimitiveComponent.SetOwnerNoSee` (`/Game/_Marvelmaster_infinite_reactive_water_/ThirdPersonBP/Blueprints/WaterTPCharacter.test` _aswater_tpcharacter) true)
      (`PrimitiveComponent.SetOwnerNoSee` _underwatercube true)
      (bind _returnvalue (`PrimitiveComponent.CreateDynamicMaterialInstance` _underwatercube 0 "/Game/_Marvelmaster_Waterline_and_Volume/Materials/X_ComplexDynamicWaterline/X_WaterLineCubeDynamic_mat.X_WaterLineCubeDynamic_mat" "None"))
      (set `self.dynmat` _returnvalue)
      (bind _outactors (`GameplayStatics.GetAllActorsOfClass` "/Game/_Marvelmaster_infinite_reactive_water_/Blueprints/WaterBody_BP0.WaterBody_BP0_C"))
      ;[1 1 1] for some reason needs to update all the time in packed project
      (`Timeline|Timeline_0` :!via `PlayFromStart`
        (:`Update`
          (`MaterialInstanceDynamic.SetTextureParameterValue` (`self.dynmat`) "Heightfield" (`/Game/_Marvelmaster_infinite_reactive_water_/Blueprints/WaterBody_BP0.height` (`|GetArrayItem` _outactors))))))
    (:`then_1`
      (`KismetSystemLibrary.K2_SetTimer` null "xxx" 0.01 true)
      (`self.xxx`)
      (`SceneComponent.K2_AttachToComponent` _clipplaneoffsetter (`self.GetComponentByClass` (`GameplayStatics.GetPlayerCharacter` 0) "/Script/Engine.CameraComponent") "None" "SnapToTarget" "SnapToTarget" "SnapToTarget" false)
      ;[1 1 1] local offset needed to match clip plane
      (`SceneComponent.K2_AddLocalOffset` _clipplaneoffsetter (10.0 0.0 0.0) false false))))

(event `self.ReceiveTick`
  (params (DeltaSeconds :type "Float (single-precision)"))
  (bind _wavecapture (`self.WaveCapture`))
  (bind _wavecapture_2 (`self.WaveCapture`))
  (bind _playercameramanager (`PlayerController.PlayerCameraManager` (`GameplayStatics.GetPlayerController` 0)))
  (`|ExecutionSequence`
    (:`then_0`
      (`KismetSystemLibrary.Delay` 0.05)
      (if (<= (`self.GetDistanceTo` _playercameramanager) 1100.0)
        (`/Engine/EditorBlueprintResources/StandardMacros.DoOnce` false :!label _label
          (:`Completed`
            (`SceneComponent.K2_AttachToComponent` _wavecapture_2 (`PlayerCameraManager.TransformComponent` _playercameramanager) "None" "SnapToTarget" "SnapToTarget" "SnapToTarget" true)
            ;[1 1 1] needed to use multiple of these blueprints in world
            (`ActorComponent.Activate` _wavecapture false)
            (goto _label_2 :!via `Reset`)))
        (else
          (`/Engine/EditorBlueprintResources/StandardMacros.DoOnce` false :!label _label_2
            (:`Completed`
              (`SceneComponent.K2_DetachFromComponent` _wavecapture_2 "KeepRelative" "KeepRelative" "KeepRelative" true)
              (`ActorComponent.Deactivate` _wavecapture)
              (`KismetSystemLibrary.Delay` 1.0)
              (`KismetRenderingLibrary.ClearRenderTarget2D` "/Game/_Marvelmaster_Waterline_and_Volume/Materials/3_ComplexWaterline/3_ComplexWaterLine_RT.3_ComplexWaterLine_RT")
              (goto _label :!via `Reset`))))))))

(event `xxx`
  (bind _underwatercube (`self.UnderWaterCube`))
  (bind (_returnvalue_location _returnvalue_rotation) (`KismetMathLibrary.BreakTransform` (`SceneComponent.K2_GetComponentToWorld` (`self.ClipPlaneOffsetter`))))
  (bind _returnvalue (`KismetMathLibrary.FTrunc` (.z _returnvalue_location)))
  (bind _returnvalue_2 (`KismetMathLibrary.Conv_IntToDouble` _returnvalue))
  (set `self.Cam Angle` _returnvalue)
  (if (<= _returnvalue_2 920.0)
    (`SceneComponent.K2_SetWorldTransform` _underwatercube (`KismetMathLibrary.MakeTransform` (`KismetMathLibrary.MakeVector` (.x _returnvalue_location) (.y _returnvalue_location) (+ (.z _returnvalue_location) 50.0)) (`KismetMathLibrary.MakeRotator` 0.0 0.0 (.yaw _returnvalue_rotation))) false false)
    (else
      (if (> _returnvalue_2 1050.0)
        (set `self.PlaneMaskScale` 0.0)
        (else
          (set `self.PlaneMaskScale` 1.0)))
      (`SceneComponent.K2_SetWorldTransform` _underwatercube (`KismetMathLibrary.MakeTransform` (`KismetMathLibrary.MakeVector` (.x _returnvalue_location) (.y _returnvalue_location) (`self.WaterLevel`)) (`KismetMathLibrary.MakeRotator` 0.0 0.0 (.yaw _returnvalue_rotation)) (`KismetMathLibrary.Conv_DoubleToVector` (`self.PlaneMaskScale`))) false false))))

(fn `UserConstructionScript`)